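; BP_Arrow is a direction helper that follows the ball each tick, steering ball direction and camera for the possessed player.
; Input offsets a red target that the black arrow faces, while the blue arrow faces the player.
; Animation curves and DoOnce gates time when green (ball direction) snaps to black or shifts 45 degrees while running.
; Yellow (player main direction) copies green on animation events, and the spring-arm camera smoothly trails green.
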(event `self.ReceiveTick`
  (params (DeltaSeconds :type "Float (single-precision)"))
  (bind _get_pawn_bp (`self.Get Pawn BP`))
  (bind _analog_force (`self.Analog force`))
  (bind _springarm_camera (`self.SpringArm Camera`))
  (bind (_returnvalue_roll _returnvalue_pitch _returnvalue_yaw) (`KismetMathLibrary.BreakRotator` (`SceneComponent.K2_GetComponentRotation` (`self.GreenArrow_BallDirection`))))
  (bind _asbp_player (cast `/Game/BallControl041/Blueprints/SoccerPlayer/BP_Player` (`GameplayStatics.GetPlayerPawn` 0)))
  (set `self.Get Pawn BP` _asbp_player)
  (bind _outactors (`GameplayStatics.GetAllActorsOfClass` "/Game/BallControl041/Blueprints/Ball/BP_Ball.BP_Ball_C"))
  (set `self.Ball_BP` (`|GetArrayItem` _outactors))
  (`self.K2_SetActorLocation` (`SceneComponent.K2_GetComponentLocation` (`/Game/BallControl041/Blueprints/Ball/BP_Ball.Sphere_physics` (`self.Ball_BP`))))
  (`SceneComponent.K2_SetRelativeLocation` (`self.RedTarget ControllerDirection`) (`KismetMathLibrary.MakeVector` (* (`/Game/BallControl041/Blueprints/SoccerPlayer/BP_Player.Get Vertical axis` _get_pawn_bp) _analog_force) (* (`/Game/BallControl041/Blueprints/SoccerPlayer/BP_Player.Get Horizontal axis` _get_pawn_bp) _analog_force)) false false)
  (`self.Controllers Event`)
  (`self.BlackArrow LookAt Event`) ; Arrow will follow Red Target Analog
  (`self.Set BlueArrow LookAt Event`)
  (`self.Setup GreenArrow BallDirection Event` :!pinned true) ; GreenArrow Direction
  (`self.Change GreenArrow Direction Event`) ; Change GreenArrow direction when player is with Ball
  (`self.Limit GreenArrow to 45 Event`)
  (`self.Limit GreenArrow Less45 Event`)
  (`SceneComponent.K2_SetWorldRotation` _springarm_camera (`KismetMathLibrary.RInterpTo` (`SceneComponent.K2_GetComponentRotation` _springarm_camera) (`KismetMathLibrary.MakeRotator` _returnvalue_roll _returnvalue_pitch (+ _returnvalue_yaw 180.0)) (`GameplayStatics.GetWorldDeltaSeconds`) 8.0) false false)
  ;[1 1 1] Set (YellowArrow) just in Animation Events
  (bind _player_possessed (`self.Get Player Possessed`))
  (add `/Game/BallControl041/Blueprints/SoccerPlayer/BP_Player_Anim.MainPosition_Direction_Dispatcher` (`/Game/BallControl041/Blueprints/SoccerPlayer/BP_Player.Player_AnimBP` _player_possessed) (delegate `MainDirection_Dispat_Event`)))

(event `MainDirection_Dispat_Event`
  (bind (_returnvalue_roll _returnvalue_pitch _returnvalue_yaw) (`KismetMathLibrary.BreakRotator` (`SceneComponent.K2_GetComponentRotation` (`self.GreenArrow_BallDirection`))))
  ;[1 1 1] Set (YellowArrow) just in Animation Events
  (set `self.YellowArrow Player_MainDirection` _returnvalue_yaw))

(event `Set BlueArrow LookAt Event`
  ;[1 1 1] Blue Arrow will look at to Player
  (bind _player_possessed (`self.Get Player Possessed`))
  (if (and (`/Game/BallControl041/Blueprints/SoccerPlayer/BP_Player.Player Possessed` _player_possessed) (not (`/Game/BallControl041/Blueprints/SoccerPlayer/BP_Player.Keep Ball` _player_possessed)))
    (`SceneComponent.K2_SetWorldRotation` (`self.BlueArrow(LookPlayer)`) (`KismetMathLibrary.MakeRotator` 0.0 0.0 (.yaw (`KismetMathLibrary.FindLookAtRotation` (`SceneComponent.K2_GetComponentLocation` (`self.BlueArrow(LookPlayer)`)) (`SceneComponent.K2_GetComponentLocation` (`Actor.RootComponent` _player_possessed))))) false false)))

(event `Set Arrow DeltaRotator Event`
  (bind (_returnvalue_roll _returnvalue_pitch _returnvalue_yaw) (`KismetMathLibrary.BreakRotator` (`SceneComponent.K2_GetComponentRotation` (`self.BlueArrow(LookPlayer)`))))
  ;[1 1 1] BlueArrow DeltaRotation
  (bind _player_possessed (`self.Get Player Possessed`))
  (set `self.Arrow DeltaRotator` (.yaw (`KismetMathLibrary.NormalizedDeltaRotator` (`KismetMathLibrary.MakeRotator` 0.0 0.0 (- _returnvalue_yaw 90.0)) (`self.K2_GetActorRotation` _player_possessed)))))

(event `BlackArrow LookAt Event`
  (bind _get_pawn_bp (`self.Get Pawn BP`))
  (bind _get_horizontal_axis (`/Game/BallControl041/Blueprints/SoccerPlayer/BP_Player.Get Horizontal axis` _get_pawn_bp))
  (bind _get_vertical_axis (`/Game/BallControl041/Blueprints/SoccerPlayer/BP_Player.Get Vertical axis` _get_pawn_bp))
  (bind (_returnvalue_roll _returnvalue_pitch _returnvalue_yaw) (`KismetMathLibrary.BreakRotator` (`KismetMathLibrary.FindLookAtRotation` (`SceneComponent.K2_GetComponentLocation` (`self.BlackArrow(Analog) Ref`)) (`SceneComponent.K2_GetComponentLocation` (`self.RedTarget ControllerDirection`)))))
  ;[1 1 1] BlackArrow will look at to (RedTarget) controlled by Gamepad Analog and Keyboard
  (if (or (< _get_horizontal_axis -0.2) (> _get_horizontal_axis 0.2) (> _get_vertical_axis 0.2) (< _get_vertical_axis -0.2))
    (`SceneComponent.K2_SetWorldRotation` (`self.BlackArrow(Analog) Ref`) (`KismetMathLibrary.MakeRotator` 0.0 0.0 _returnvalue_yaw) false false)))

(event `Controllers Event`
  ;[1 1 1] Get Joystick and Keyboard
  (set `self.Horizontal Axis` (+ (`self.GetInputAxisValue`) (`self.GetInputAxisValue`)))
  (set `self.Vertical Axis` (+ (`self.GetInputAxisValue`) (`self.GetInputAxisValue`))))

(event `Set Player Variables Event`
  (bind _player_possessed (`self.Get Player Possessed`))
  (set `self.PlayerDirection Ref` (`/Game/BallControl041/Blueprints/SoccerPlayer/BP_Player.Player Direction Ref` _player_possessed))
  (set `self.speed animation Ref` (`/Game/BallControl041/Blueprints/SoccerPlayer/BP_Player.speed animation Ref` _player_possessed))
  (set `self.ballVelocity` (`/Game/BallControl041/Blueprints/SoccerPlayer/BP_Player.ballVelocity` _player_possessed)))

(fn `Get Player KeepBall`
  (returns (`Players KeepBall` :type "/Game/BallControl041/Blueprints/SoccerPlayer/BP_Player Object Reference"))
  (bind _outactors (`GameplayStatics.GetAllActorsOfClass` "/Game/BallControl041/Blueprints/SoccerPlayer/BP_Player.BP_Player_C"))
  (for _array_element _outactors
    (if (`/Game/BallControl041/Blueprints/SoccerPlayer/BP_Player.Player Possessed` _array_element)
      (return _array_element))))

(fn `Get Player Possessed`
  (returns (`Player Possessed` :type "/Game/BallControl041/Blueprints/SoccerPlayer/BP_Player Object Reference"))
  ;[1 1 1] Get the Player that is with the variable (Is withBall) = TRUE
  (bind _outactors (`GameplayStatics.GetAllActorsOfClass` "/Game/BallControl041/Blueprints/SoccerPlayer/BP_Player.BP_Player_C"))
  (for _array_element _outactors
    (if (`/Game/BallControl041/Blueprints/SoccerPlayer/BP_Player.Player Possessed` _array_element)
      (return _array_element))))

(fn `Get Player WithBall`
  (returns (`Player withBall` :type "/Game/BallControl041/Blueprints/SoccerPlayer/BP_Player Object Reference"))
  ;[1 1 1] Get the Player that is with the variable (Is withBall) = TRUE
  (bind _outactors (`GameplayStatics.GetAllActorsOfClass` "/Game/BallControl041/Blueprints/SoccerPlayer/BP_Player.BP_Player_C"))
  (for _array_element _outactors
    (if (`/Game/BallControl041/Blueprints/SoccerPlayer/BP_Player.Is withBall?` _array_element)
      (return _array_element))))

(fn `ReachBall Location`
  (params (Forward :type "Float (double-precision)") (Right :type "Float (double-precision)"))
  (bind _reachball (`self.ReachBall`))
  (bind (_relativelocation_x _relativelocation_y _relativelocation_z) (`KismetMathLibrary.BreakVector` (`SceneComponent.RelativeLocation` _reachball)))
  ;[1 1 1] Set ReahBall RelativeLocation
  (bind _output_get (set `self.ReachBall Forward` Forward))
  (bind _output_get_2 (set `self.ReachBall Right` Right))
  (`SceneComponent.K2_SetRelativeLocation` _reachball (`KismetMathLibrary.MakeVector` _output_get _output_get_2 _relativelocation_z) false false))

(fn `UserConstructionScript`)