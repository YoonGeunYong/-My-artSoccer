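; Soccer ball actor that handles possession, kick and pass motion, and the camera following it.
; Tick copies input flags to the possessed player, tracks speed and goal Y distance, and interpolates the camera with zoom and numpad rotation.
; Overlaps flag possession, but the physics-disable event they call is empty.
; Callable events switch mass and damping, or launch the ball toward the arrow, goal target or pass guide via velocity, force or offset.
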(event `self.ReceiveBeginPlay`
  (bind _outactors (`GameplayStatics.GetAllActorsOfClass` "/Game/BallControl041/Blueprints/Ball/BP_Arrow.BP_Arrow_C"))
  (set `self.Arrow BP` (`|GetArrayItem` _outactors))
  (`self.Iniciate CameraView Event`)
  (bind _outactors_2 (`GameplayStatics.GetAllActorsOfClass` "/Game/BallControl041/Blueprints/Goal/BP_Target.BP_Target_C"))
  (set `self.GoalTarget BP` (`|GetArrayItem` _outactors_2)) ; Set Goal Target to Get
  (bind _asbp_player (cast `/Game/BallControl041/Blueprints/SoccerPlayer/BP_Player` (`GameplayStatics.GetPlayerPawn` 0)))
  (set `self.Get Pawn` _asbp_player)
  (`self.Iniciate CameraView Event` :!pinned true) ; Camera View
  (if (`self.Enable Controller`)
    ;[1 1 1] Enable Player Controller
    (bind _outactors_3 (`GameplayStatics.GetAllActorsOfClass` "/Game/BallControl041/Blueprints/SoccerPlayer/BP_Player.BP_Player_C"))
    (for _array_element _outactors_3
      (set `/Game/BallControl041/Blueprints/SoccerPlayer/BP_Player.Enable Controller` true _array_element))))

(event `self.ReceiveTick`
  (params (DeltaSeconds :type "Float (single-precision)"))
  (set `self.DeltaSeconds` DeltaSeconds)
  (bind _player_possessed (`/Game/BallControl041/Blueprints/Ball/BP_Arrow.Get Player Possessed` (`self.Arrow BP`)))
  (set `/Game/BallControl041/Blueprints/SoccerPlayer/BP_Player.Enable BallPass` (`self.Enable BallPass`) _player_possessed)
  (set `/Game/BallControl041/Blueprints/SoccerPlayer/BP_Player.Enable Kick Input` (`self.Enable Kick Input`) _player_possessed)
  (set `/Game/BallControl041/Blueprints/SoccerPlayer/BP_Player.Enable Crossing` (`self.Enable Crossing`) _player_possessed)
  (`self.Goal Distance Y Event`)
  (`self.SetCameraTransform Event` :!pinned true) ; Camera
  (bind _output_get (set `self.ball_vector` (`SceneComponent.GetComponentVelocity` (`self.Sphere_physics`))))
  (set `self.ballVelocity` (`KismetMathLibrary.VSize` (`KismetMathLibrary.MakeVector` (.x _output_get) (.y _output_get)))))

(event `self.BallCollision.OnComponentBeginOverlap`
  (params (OverlappedComponent :type "PrimitiveComponent Object Reference") (OtherActor :type "Actor Object Reference") (OtherComp :type "PrimitiveComponent Object Reference") (OtherBodyIndex :type Integer) (bFromSweep :type Boolean) (SweepResult :type "HitResult Structure (by ref)"))
  ;[1 1 1] Ball Collision
  (bind _asbp_player (cast `/Game/BallControl041/Blueprints/SoccerPlayer/BP_Player` OtherActor)
    (:`then`
      _)
    (:`CastFailed`
      (bind _asbpc_goal_keeper (cast `/Game/CustomBlueprint/BPC_GoalKeeper` OtherActor))))
  (if (and (`/Game/BallControl041/Blueprints/SoccerPlayer/BP_Player.Keep Ball` _asbp_player) (== (`/Game/BallControl041/Blueprints/SoccerPlayer/BP_Player.capsuleFootCollision_Kick` _asbp_player) OtherComp))
    (set `self.ball hit` true :!label _label)
    (set `/Game/BallControl041/Blueprints/SoccerPlayer/BP_Player.Is withBall?` true _asbp_player)
    (set `/Game/BallControl041/Blueprints/SoccerPlayer/BP_Player.Keep Ball` false _asbp_player)
    ;[1 1 1] Disable Ball Physics
    (`self.Disable BallPhysics Events`)
    (elif (== (`Character.CapsuleComponent` _asbpc_goal_keeper) OtherComp)
      (goto _label))))

(event `Iniciate CameraView Event`
  ;[1 1 1] Camera will follow the Ball we can also change the location of the Camera
  (bind _outactors (`GameplayStatics.GetAllActorsOfClass` "/Game/BallControl041/Blueprints/BP_CameraActor.BP_CameraActor_C"))
  (`PlayerController.SetViewTargetWithBlend` (`GameplayStatics.GetPlayerController` 0) (`|GetArrayItem` _outactors) 0.0 "VTBlend_Cubic" 0.0 false :!label _label))

(event `SetCameraTransform Event`
  (bind _right_analogic_up_increment (`self.Right Analogic up Increment`))
  (bind _deltaseconds (`self.DeltaSeconds`))
  (bind _get_pawn (`self.Get Pawn`))
  (bind (_camera_position_x _camera_position_y _camera_position_z) (`KismetMathLibrary.BreakVector` (`self.Camera_Position`)))
  ;[1 1 1] Camera will follow the Ball we can also change the location of the Camera
  (if (> (`/Game/BallControl041/Blueprints/SoccerPlayer/BP_Player.Right analogic Up` _get_pawn) 0.0)
    (set `self.Right Analogic up Increment` (`KismetMathLibrary.FInterpTo` _right_analogic_up_increment 200.0 _deltaseconds 1.0))
    (elif (< (`/Game/BallControl041/Blueprints/SoccerPlayer/BP_Player.Right analogic Down` _get_pawn) 0.0)
      (set `self.Right Analogic up Increment` (`KismetMathLibrary.FInterpTo` _right_analogic_up_increment -200.0 _deltaseconds 1.0))))
  (bind _output (`|GetArrayItem` (stale `Iniciate CameraView Event` _outactors)))
  (`self.K2_SetActorTransform` _output (`KismetMathLibrary.MakeTransform` (.location (`KismetMathLibrary.TInterpTo` (`SceneComponent.K2_GetComponentToWorld` (`CameraActor.CameraComponent` _output)) (`KismetMathLibrary.MakeTransform` (`KismetMathLibrary.MakeVector` (+ _camera_position_x (.x (.location (`SceneComponent.GetRelativeTransform` (`self.Sphere_physics`)))) (* (`KismetMathLibrary.Conv_IntToDouble` (`self.MouseWheel`)) 2.0) (* (`self.Right Analogic up Increment`) 5.0)) (+ _camera_position_y (.y (.location (`SceneComponent.GetRelativeTransform` (`self.Sphere_physics`)))) (* (`KismetMathLibrary.Conv_IntToDouble` (`self.Mouse Wheel_FreeKick`)) 2.0)) (+ _camera_position_z (* (`KismetMathLibrary.Conv_IntToDouble` (`self.MouseWheel`)) -0.5) (* (`self.Right Analogic up Increment`) -1.0))) (`self.Camera Rotation Macro`)) (`GameplayStatics.GetWorldDeltaSeconds`) 4.0)) (.rotation (`KismetMathLibrary.TInterpTo` (`SceneComponent.K2_GetComponentToWorld` (`CameraActor.CameraComponent` _output)) (`KismetMathLibrary.MakeTransform` (`KismetMathLibrary.MakeVector` (+ _camera_position_x (.x (.location (`SceneComponent.GetRelativeTransform` (`self.Sphere_physics`)))) (* (`KismetMathLibrary.Conv_IntToDouble` (`self.MouseWheel`)) 2.0) (* (`self.Right Analogic up Increment`) 5.0)) (+ _camera_position_y (.y (.location (`SceneComponent.GetRelativeTransform` (`self.Sphere_physics`)))) (* (`KismetMathLibrary.Conv_IntToDouble` (`self.Mouse Wheel_FreeKick`)) 2.0)) (+ _camera_position_z (* (`KismetMathLibrary.Conv_IntToDouble` (`self.MouseWheel`)) -0.5) (* (`self.Right Analogic up Increment`) -1.0))) (`self.Camera Rotation Macro`)) (`GameplayStatics.GetWorldDeltaSeconds`) 4.0))) false false)
  (`self.Camera Rotation Event`))

(event `Key|One`
  (params (Key :type "Key Structure"))
  ;[1 1 1] Camera will follow the Ball we can also change the location of the Camera
  (:`Pressed`
    (goto _label)))

(event `Camera Rotation Event`
  (bind _camera_rotation_z (`self.Camera Rotation Z`))
  (bind _camera_rotation_y (`self.Camera Rotation Y`))
  (bind _camera_rotation_z_2 (`self.Camera Rotation Z`))
  (bind _camera_rotation_y_2 (`self.Camera Rotation Y`))
  ;[1 1 1] Change Camera Rotation with Keyboard
  (if (`self.Num 8`)
    (set `self.Camera Rotation Y` (`KismetMathLibrary.FInterpTo` _camera_rotation_y_2 (+ _camera_rotation_y_2 20.0) (`self.DeltaSeconds`) 1.0))
    (elif (`self.Num 2`)
      (set `self.Camera Rotation Y` (`KismetMathLibrary.FInterpTo` _camera_rotation_y (+ _camera_rotation_y -20.0) (`self.DeltaSeconds`) 1.0))
      (elif (`self.Num 6`)
        (set `self.Camera Rotation Z` (`KismetMathLibrary.FInterpTo` _camera_rotation_z_2 (+ _camera_rotation_z_2 20.0) (`self.DeltaSeconds`) 1.0))
        (elif (`self.Num 4`)
          (set `self.Camera Rotation Z` (`KismetMathLibrary.FInterpTo` _camera_rotation_z (+ _camera_rotation_z -20.0) (`self.DeltaSeconds`) 1.0)))))))

(event `Key|MouseScrollUp` :overrideparent false
  (params (Key :type "Key Structure"))
  ;[1 1 1] Set Mouse Wheel
  (:`Pressed`
    (if (`self.FreeKick`)
      (bind _result (`/Engine/EditorBlueprintResources/StandardMacros.IncrementInt` (+ (`self.Mouse Wheel_FreeKick`) 40))
        (:`  `
          (set `self.Mouse Wheel_FreeKick` (`KismetMathLibrary.Min` _result 150))))
      (else
        (bind _result_2 (`/Engine/EditorBlueprintResources/StandardMacros.IncrementInt` (+ (`self.MouseWheel`) 40))
          (:`  `
            (set `self.MouseWheel` (`KismetMathLibrary.Min` _result_2 500))))))))

(event `Key|MouseScrollDown` :overrideparent false
  (params (Key :type "Key Structure"))
  ;[1 1 1] Set Mouse Wheel
  (:`Pressed`
    (if (`self.FreeKick`)
      (bind _result (`/Engine/EditorBlueprintResources/StandardMacros.IncrementInt` (+ (`self.Mouse Wheel_FreeKick`) -40))
        (:`  `
          (set `self.Mouse Wheel_FreeKick` (`KismetMathLibrary.Max` _result -100))))
      (else
        (bind _result_2 (`/Engine/EditorBlueprintResources/StandardMacros.DecrementInt` (+ (`self.MouseWheel`) -40))
          (:`  `
            (set `self.MouseWheel` (`KismetMathLibrary.Max` _result_2 -400))))))))

(event `self.Sphere_physics.OnComponentBeginOverlap`
  (params (OverlappedComponent :type "PrimitiveComponent Object Reference") (OtherActor :type "Actor Object Reference") (OtherComp :type "PrimitiveComponent Object Reference") (OtherBodyIndex :type Integer) (bFromSweep :type Boolean) (SweepResult :type "HitResult Structure (by ref)"))
  (bind _returnvalue (`GameplayStatics.GetActorOfClass` "/Game/CustomBlueprint/BPC_GoalKeeper.BPC_GoalKeeper_C"))
  (if (== OtherActor (`self.GetOwner` _returnvalue))
    (`KismetSystemLibrary.PrintString` "asd")))

(event `Impulse ball Event`
  (bind (_returnvalue_x _returnvalue_y) (`KismetMathLibrary.BreakVector` (* (`self.Ball Direction`) (* (`self.Ball Impulse`) (`self.DeltaSeconds`)))))
  ;[1 1 1] Ball Impulse to Turn Animations
  (`SceneComponent.K2_AddWorldOffset` (`self.Sphere_physics`) (`KismetMathLibrary.MakeVector` _returnvalue_x _returnvalue_y) false false))

(event `ImpulseBall Goal Event`
  ;[1 1 1] Ball Impulse to Goal Target
  (bind _output_get (set `self.TargetGoal Position` (`SceneComponent.K2_GetComponentLocation` (`/Game/BallControl041/Blueprints/Goal/BP_Target.Target` (`self.GoalTarget BP`)))))
  (set `self.Ball Impulse` 5000.0)
  (`PrimitiveComponent.AddForce` (`self.Sphere_physics`) (`KismetMathLibrary.MakeVector` (.x (* (`KismetMathLibrary.MakeVector` (.x (`KismetMathLibrary.Normal` (- _output_get (`SceneComponent.K2_GetComponentLocation` (`self.Sphere_physics`))))) (.y (`KismetMathLibrary.Normal` (- _output_get (`SceneComponent.K2_GetComponentLocation` (`self.Sphere_physics`)))))) (* (`self.Ball Impulse`) 2.0))) (.y (* (`KismetMathLibrary.MakeVector` (.x (`KismetMathLibrary.Normal` (- _output_get (`SceneComponent.K2_GetComponentLocation` (`self.Sphere_physics`))))) (.y (`KismetMathLibrary.Normal` (- _output_get (`SceneComponent.K2_GetComponentLocation` (`self.Sphere_physics`)))))) (* (`self.Ball Impulse`) 2.0))) 3500.0) "None" true))

(event `Goal Distance Y Event`
  (bind (_returnvalue_x _returnvalue_y) (`KismetMathLibrary.BreakVector` (- (`SceneComponent.K2_GetComponentLocation` (`Actor.RootComponent` (`self.GoalTarget BP`))) (`SceneComponent.K2_GetComponentLocation` (`self.Sphere_physics`)))))
  ;[1 1 1] Calculate the distance between the ball and the GoalTarget Root Component
  (set `self.Goal_Distance Y` _returnvalue_y))

(event `Ball Physics Linear Event`
  (bind (_returnvalue_x _returnvalue_y) (`KismetMathLibrary.BreakVector` (* (`KismetMathLibrary.Normal` (`SceneComponent.GetForwardVector` (`/Game/BallControl041/Blueprints/Ball/BP_Arrow.GreenArrow_BallDirection` (`self.Arrow BP`)))) (+ (`self.Ball Force GoalTarget`) (`self.DeltaSeconds`)))))
  (`PrimitiveComponent.SetAllPhysicsLinearVelocity` (`self.Sphere_physics`) (`KismetMathLibrary.MakeVector` _returnvalue_x _returnvalue_y (`self.Ball Z axis`)) false))

(event `BallPhysics TargetPass Event`
  (bind _outactors (`GameplayStatics.GetAllActorsOfClass` "/Game/BallControl041/Blueprints/Ball/PassGuide_BP.PassGuide_BP_C"))
  (bind _output_get (set `self.Player Loc` (`/Game/BallControl041/Blueprints/Ball/PassGuide_BP.Player_Location` (`|GetArrayItem` _outactors))))
  (`PrimitiveComponent.SetAllPhysicsLinearVelocity` (`self.Sphere_physics`) (`KismetMathLibrary.MakeVector` (.x (* (`KismetMathLibrary.Normal` (- _output_get (`SceneComponent.K2_GetComponentLocation` (`self.Sphere_physics`)))) (+ (`self.Pass Force`) (`self.DeltaSeconds`)))) (.y (* (`KismetMathLibrary.Normal` (- _output_get (`SceneComponent.K2_GetComponentLocation` (`self.Sphere_physics`)))) (+ (`self.Pass Force`) (`self.DeltaSeconds`)))) (`self.Ball Z axis`)) false))

(event `BallPhysics GoalTarget Event`
  (bind _returnvalue (`KismetMathLibrary.MakeVector` (.x (* (`KismetMathLibrary.Normal` (- (`SceneComponent.K2_GetComponentLocation` (`/Game/BallControl041/Blueprints/Goal/BP_Target.Target` (`self.GoalTarget BP`))) (`SceneComponent.K2_GetComponentLocation` (`self.Sphere_physics`)))) (+ (`self.Ball Force GoalTarget`) (`self.DeltaSeconds`)))) (.y (* (`KismetMathLibrary.Normal` (- (`SceneComponent.K2_GetComponentLocation` (`/Game/BallControl041/Blueprints/Goal/BP_Target.Target` (`self.GoalTarget BP`))) (`SceneComponent.K2_GetComponentLocation` (`self.Sphere_physics`)))) (+ (`self.Ball Force GoalTarget`) (`self.DeltaSeconds`)))) (`self.Ball Z axis`)))
  (`PrimitiveComponent.SetAllPhysicsLinearVelocity` (`self.Sphere_physics`) _returnvalue false)
  (if (`/Game/BallControl041/Blueprints/Goal/BP_Target.ClashGoalKeeper` (`self.GoalTarget BP`))
    (set `self.GetBallVelocity` _returnvalue)))

(event `Ball Pass Physics Event`
  (bind _sphere_physics (`self.Sphere_physics`))
  ;[1 1 1] Change the ball physics to pass
  (`PrimitiveComponent.SetMassOverrideInKg` _sphere_physics "None" 0.1 true)
  (`PrimitiveComponent.SetLinearDamping` _sphere_physics 0.01)
  (`PrimitiveComponent.SetAngularDamping` _sphere_physics 1.0))

(event `WalkBall Physics Event`
  (bind _sphere_physics (`self.Sphere_physics`))
  ;[1 1 1] Change the ball physics to pass
  (`PrimitiveComponent.SetMassOverrideInKg` _sphere_physics "None" 50.0 true)
  (`PrimitiveComponent.SetLinearDamping` _sphere_physics 0.6)
  (`PrimitiveComponent.SetAngularDamping` _sphere_physics 0.0))

(event `Disable BallPhysics Events`
  ;[1 1 1] Disable Ball Physics
)

(event `Key|NumPadEight`
  (params (Key :type "Key Structure"))
  ;[1 1 1] Num 8
  (:`Pressed`
    (set `self.Num 8` true))
  (:`Released`
    (set `self.Num 8` false)))

(event `Key|NumPadFour`
  (params (Key :type "Key Structure"))
  ;[1 1 1] Num 4
  (:`Pressed`
    (set `self.Num 4` true))
  (:`Released`
    (set `self.Num 4` false)))

(event `Key|NumPadTwo`
  (params (Key :type "Key Structure"))
  ;[1 1 1] Num 9
  (:`Pressed`
    (set `self.Num 2` true))
  (:`Released`
    (set `self.Num 2` false)))

(event `Key|NumPadSix`
  (params (Key :type "Key Structure"))
  ;[1 1 1] Num 6
  (:`Pressed`
    (set `self.Num 6` true))
  (:`Released`
    (set `self.Num 6` false)))

(fn `UserConstructionScript`)