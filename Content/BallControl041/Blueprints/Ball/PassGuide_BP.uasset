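; Pass guide for a ball game that aims passes and crosses and picks the receiving player.
; Each Tick it follows the ball carrier while not passing, using an input-driven red sphere to steer the white arrow.
; Holding pass or cross interpolates the target outward; release selects the player nearest it, flags them possessed and pins the target to them.
; Animation events from the player's AnimBP clear and re-arm the selection.
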(event `self.ReceiveBeginPlay`
  (bind _asbp_player (cast `/Game/BallControl041/Blueprints/SoccerPlayer/BP_Player` (`GameplayStatics.GetPlayerPawn` 0)))
  (set `self.Get Pawn BP` _asbp_player)
  (bind _outactors (`GameplayStatics.GetAllActorsOfClass` "/Game/BallControl041/Blueprints/Ball/BP_Ball.BP_Ball_C"))
  (set `self.Ball BP` (`|GetArrayItem` _outactors))
  (bind _outactors_2 (`GameplayStatics.GetAllActorsOfClass` "/Game/BallControl041/Blueprints/SoccerPlayer/BP_Player.BP_Player_C"))
  (for _array_element _outactors_2
    (`KismetArrayLibrary.Array_Add` (`self.Find Actors Array`) _array_element)))

(event `Clear Actors Event`
  ;[1 1 1] Get All Actors without the Ball
  (`KismetArrayLibrary.Array_Clear` (`self.Player Distance`))
  (`KismetArrayLibrary.Array_Clear` (`self.ActorClosest Array`))
  (set `self.Closest Player Ref` null))

(event `self.ReceiveTick`
  (params (DeltaSeconds :type "Float (single-precision)"))
  (bind _ball_bp (`self.Ball BP`))
  (if (or (`/Game/BallControl041/Blueprints/Ball/BP_Ball.Enable BallPass` _ball_bp) (`/Game/BallControl041/Blueprints/Ball/BP_Ball.Enable Crossing` _ball_bp))
    (`self.Follow Player Event`)
    (`self.Controller Event` :!pinned true) ; Controller
    (`self.WhiteArrow Look Event`)
    ;[1 1 1] Adjust (WhiteARrow) Direction to Player Direction
    (`self.WhiteArrow Direction Event`)
    (`self.TargetPass Event`)
    ;[1 1 1] Get All Actors without the Ball
    (bind _player_possessed (`self.Get Player Possessed`))
    (bind _player_animbp (`/Game/BallControl041/Blueprints/SoccerPlayer/BP_Player.Player_AnimBP` _player_possessed))
    (add `/Game/BallControl041/Blueprints/SoccerPlayer/BP_Player_Anim.BallPass_GetClosestPlayer_Event` _player_animbp (delegate `Clear Actors Event`))
    (add `/Game/BallControl041/Blueprints/SoccerPlayer/BP_Player_Anim.Reset BallPass Animation_Event` _player_animbp (delegate `Reset Get Actors Event`))
    (bind _player_possessed_2 (`/Game/BallControl041/Blueprints/SoccerPlayer/BP_Player.Player Possessed` _player_possessed))
    (if (or (and _player_possessed_2 (`/Game/BallControl041/Blueprints/SoccerPlayer/BP_Player.BallPass Input` _player_possessed) (not (`/Game/BallControl041/Blueprints/SoccerPlayer/BP_Player.E Key` _player_possessed))) (and _player_possessed_2 (not (`/Game/BallControl041/Blueprints/SoccerPlayer/BP_Player.R Key` _player_possessed)) (`/Game/BallControl041/Blueprints/SoccerPlayer/BP_Player.Crossing Input` _player_possessed)))
      (`/Engine/EditorBlueprintResources/StandardMacros.DoOnce` false :!label _label
        (:`Completed`
          (set `self.TargetPass Follow Player` true)
          (`KismetArrayLibrary.Array_Clear` (`self.Player Distance`))
          (`KismetArrayLibrary.Array_Clear` (`self.ActorClosest Array`))
          (bind _outactors (`GameplayStatics.GetAllActorsOfClass` "/Game/BallControl041/Blueprints/SoccerPlayer/BP_Player.BP_Player_C"))
          (for _array_element _outactors
            (if (and (not (`/Game/BallControl041/Blueprints/SoccerPlayer/BP_Player.Player Possessed` _array_element)) (> (`/Game/BallControl041/Blueprints/SoccerPlayer/BP_Player.Ball Distance` _array_element) 210.0))
              (bind _output_get (set `self.Players Distances` (`KismetMathLibrary.VSize` (`KismetMathLibrary.MakeVector` (.x (- (`self.K2_GetActorLocation` _array_element) (`SceneComponent.K2_GetComponentLocation` (`self.TargetPass`)))) (.y (- (`self.K2_GetActorLocation` _array_element) (`SceneComponent.K2_GetComponentLocation` (`self.TargetPass`))))))))
              (`KismetArrayLibrary.Array_Add` (`self.Player Distance`) _output_get)
              (`KismetArrayLibrary.Array_Add` (`self.ActorClosest Array`) _array_element)))
          (`SceneComponent.K2_SetRelativeLocation` (`self.RedSphere_Controller`) (0.0 0.0 0.0) false false)
          (`self.Closest Player`)
          (`KismetSystemLibrary.Delay` 0.1)
          (`self.WhiteArrow Direction Event`))))))

(event `Reset Get Actors Event`
  ;[1 1 1] Get All Actors without the Ball
  (`KismetSystemLibrary.Delay` 0.7) ; Fix Buf
  (goto _label :!via `Reset`))

(event `Controller Event`
  (bind _redsphere_multiplier_location (`self.RedSphere_Multiplier_Location`))
  ;[1 1 1] RedSphere Controller
  (bind _player_possessed (`self.Get Player Possessed`))
  (bind _get_horizontal_axis (`/Game/BallControl041/Blueprints/SoccerPlayer/BP_Player.Get Horizontal axis` _player_possessed))
  (bind _get_vertical_axis (`/Game/BallControl041/Blueprints/SoccerPlayer/BP_Player.Get Vertical axis` _player_possessed))
  (if (and (`/Game/BallControl041/Blueprints/SoccerPlayer/BP_Player.E Key` _player_possessed) (or (< _get_horizontal_axis -0.2) (> _get_horizontal_axis 0.2) (> _get_vertical_axis 0.2) (< _get_vertical_axis -0.2)) (`/Game/BallControl041/Blueprints/SoccerPlayer/BP_Player.Player Possessed` _player_possessed))
    (`SceneComponent.K2_SetRelativeLocation` (`self.RedSphere_Controller`) (`KismetMathLibrary.MakeVector` (* (`/Game/BallControl041/Blueprints/SoccerPlayer/BP_Player.Get Vertical axis` _player_possessed) _redsphere_multiplier_location) (* (`/Game/BallControl041/Blueprints/SoccerPlayer/BP_Player.Get Horizontal axis` _player_possessed) _redsphere_multiplier_location)) false false)))

(event `WhiteArrow Look Event`
  (bind _get_pawn_bp (`self.Get Pawn BP`))
  (bind _get_horizontal_axis (`/Game/BallControl041/Blueprints/SoccerPlayer/BP_Player.Get Horizontal axis` _get_pawn_bp))
  (bind _get_vertical_axis (`/Game/BallControl041/Blueprints/SoccerPlayer/BP_Player.Get Vertical axis` _get_pawn_bp))
  (bind (_returnvalue_roll _returnvalue_pitch _returnvalue_yaw) (`KismetMathLibrary.BreakRotator` (`KismetMathLibrary.FindLookAtRotation` (`SceneComponent.K2_GetComponentLocation` (`self.White_Arrow`)) (`SceneComponent.K2_GetComponentLocation` (`self.RedSphere_Controller`)))))
  ;[1 1 1] WriteArrow Look at
  (bind _player_possessed (`self.Get Player Possessed`))
  (if (and (`/Game/BallControl041/Blueprints/SoccerPlayer/BP_Player.Player Possessed` _player_possessed) (`/Game/BallControl041/Blueprints/SoccerPlayer/BP_Player.BallPass Input` _player_possessed) (or (< _get_horizontal_axis -0.2) (> _get_horizontal_axis 0.2) (> _get_vertical_axis 0.2) (< _get_vertical_axis -0.2)))
    (`SceneComponent.K2_SetWorldRotation` (`self.White_Arrow`) (`KismetMathLibrary.MakeRotator` 0.0 0.0 _returnvalue_yaw) false false)))

(event `WhiteArrow Direction Event`
  ;[1 1 1] WriteArrow Look at
  (bind _player_possessed (`self.Get Player Possessed`))
  (bind _returnvalue (not (`/Game/BallControl041/Blueprints/SoccerPlayer/BP_Player.BallPass Input` _player_possessed)))
  (bind _player_possessed_2 (`/Game/BallControl041/Blueprints/SoccerPlayer/BP_Player.Player Possessed` _player_possessed))
  (bind _keep_ball (`/Game/BallControl041/Blueprints/SoccerPlayer/BP_Player.Keep Ball` _player_possessed))
  (if (or (and _returnvalue _player_possessed_2 (not _keep_ball)) (and _returnvalue _player_possessed_2 _keep_ball))
    (bind (_returnvalue_roll _returnvalue_pitch _returnvalue_yaw) (`KismetMathLibrary.BreakRotator` (`SceneComponent.K2_GetComponentRotation` (`Actor.RootComponent` _player_possessed))))
    (`SceneComponent.K2_SetWorldRotation` (`self.White_Arrow`) (`KismetMathLibrary.MakeRotator` 0.0 0.0 (+ _returnvalue_yaw 90.0)) false false)))

(event `TargetPass Event`
  ;[1 1 1] TargetPass Follow
  (`/Engine/EditorBlueprintResources/StandardMacros.IsValid` (`self.Closest Player Ref`)
    (:`Is Valid`
      (set `self.ClosestPlayer_IsValid` true)
      (`self.TargetPass FollowPlayer Event`)
      (set `self.TargetPass Follow X axis` 0.0)
      (`SceneComponent.K2_SetRelativeLocation` (`self.TargetPass_Follow`) (0.0 0.0 3.493971) false false))
    (:`Is Not Valid`
      (`self.Set Location Event`))))

(event `Pass_Animation_Event`
  (bind _player_last_location (`self.Player Last location`))
  ;[1 1 1] TargetPass Follow
  (set `self.TargetPass Follow Player` false)
  (`SceneComponent.K2_SetWorldLocation` (`self.DefaultSceneRoot`) (`KismetMathLibrary.MakeVector` (.x _player_last_location) (.y _player_last_location) 3.0) false false)
  (`SceneComponent.K2_SetWorldLocation` (`self.TargetPass`) (`KismetMathLibrary.MakeVector` (.x _player_last_location) (.y _player_last_location) 3.0) false false))

(event `Set Location Event`
  (bind _ball_bp (`self.Ball BP`))
  (bind _targetpass (`self.TargetPass`))
  (bind _returnvalue (not (`self.Lock TargetPass_Follow Location`)))
  (bind (_returnvalue_x _returnvalue_y) (`KismetMathLibrary.BreakVector` (`KismetMathLibrary.VInterpTo` (`SceneComponent.K2_GetComponentLocation` _targetpass) (`SceneComponent.K2_GetComponentLocation` (`self.TargetPass_Follow`)) (`GameplayStatics.GetWorldDeltaSeconds`) 10.0)))
  ;[1 1 1] TargetPass Follow
  (`/Engine/EditorBlueprintResources/StandardMacros.IsValid` (`self.Closest Player Ref`)
    (:`Is Not Valid`
      (bind _player_possessed (`self.Get Player Possessed`))
      (add `/Game/BallControl041/Blueprints/SoccerPlayer/BP_Player_Anim.Pass_Animation_Event` (`/Game/BallControl041/Blueprints/SoccerPlayer/BP_Player.Player_AnimBP` _player_possessed) (delegate `Pass_Animation_Event`))
      (set `self.ClosestPlayer_IsValid` false)
      (`SceneComponent.K2_SetWorldLocation` _targetpass (`KismetMathLibrary.MakeVector` _returnvalue_x _returnvalue_y 5.0) false false)
      (`SceneComponent.K2_SetRelativeLocation` (`self.TargetPass_Follow`) (`KismetMathLibrary.MakeVector` (`self.TargetPass Follow X axis`) 0.0 3.493971) false false)
      (bind _player_possessed_2 (`self.Get Player Possessed`))
      (bind _player_possessed_3 (`/Game/BallControl041/Blueprints/SoccerPlayer/BP_Player.Player Possessed` _player_possessed_2))
      (if (or (and (`/Game/BallControl041/Blueprints/SoccerPlayer/BP_Player.E Key` _player_possessed_2) _player_possessed_3 _returnvalue (`/Game/BallControl041/Blueprints/Ball/BP_Ball.Enable BallPass` _ball_bp)) (and _returnvalue _player_possessed_3 (`/Game/BallControl041/Blueprints/SoccerPlayer/BP_Player.R Key` (`self.Get Pawn BP`)) (`/Game/BallControl041/Blueprints/Ball/BP_Ball.Enable Crossing` _ball_bp)))
        (set `self.TargetPass Follow X axis` (`KismetMathLibrary.FInterpTo` (`self.TargetPass Follow X axis`) 2000.0 (`GameplayStatics.GetWorldDeltaSeconds`) 1.5))))))

(event `TargetPass FollowPlayer Event`
  (bind _returnvalue (`self.K2_GetActorLocation` (`self.Closest Player Ref`)))
  ;[1 1 1] TargetPass Follow
  (if (`self.TargetPass Follow Player`)
    (set `self.Player Last location` _returnvalue)
    (`SceneComponent.K2_SetWorldLocation` (`self.TargetPass`) (`KismetMathLibrary.MakeVector` (.x _returnvalue) (.y _returnvalue) 3.0) false false)))

(event `Follow Player Event`
  ;[1 1 1] Follow Player
  (bind _player_possessed (`self.Get Player Possessed`))
  (if (and (`/Game/BallControl041/Blueprints/SoccerPlayer/BP_Player.Player Possessed` _player_possessed) (`/Game/BallControl041/Blueprints/SoccerPlayer/BP_Player.Is withBall?` _player_possessed) (not (`/Game/BallControl041/Blueprints/SoccerPlayer/BP_Player.E Key` _player_possessed)) (not (`/Game/BallControl041/Blueprints/SoccerPlayer/BP_Player.BallPass Input` _player_possessed)))
    (bind (_returnvalue_x _returnvalue_y) (`KismetMathLibrary.BreakVector` (`SceneComponent.K2_GetComponentLocation` (`Character.Mesh` _player_possessed))))
    (`SceneComponent.K2_SetWorldLocation` (`self.DefaultSceneRoot`) (`KismetMathLibrary.MakeVector` _returnvalue_x _returnvalue_y 3.0) false false)))

(fn `Closest Player`
  ;[1 1 1] Get Closest Player that will Keep Ball or the farthest player
  (bind _asbp_player (cast `/Game/BallControl041/Blueprints/SoccerPlayer/BP_Player` (`|GetArrayItem` (`self.ActorClosest Array`) (`KismetMathLibrary.MinOfFloatArray` (`self.Player Distance`)))))
  (set `self.Closest Player Ref` _asbp_player)
  (set `self.Player_Location` (`self.K2_GetActorLocation` _asbp_player)) ; Closest Player
  (set `self.FollowGuide` true)
  (set `/Game/BallControl041/Blueprints/SoccerPlayer/BP_Player.Player Possessed` true _asbp_player)
  (set `/Game/BallControl041/Blueprints/SoccerPlayer/BP_Player.Keep Ball` true _asbp_player)
  (set `self.Player Index` 0) ; Closest Player
  (return))

(fn `Get Player Possessed`
  (returns (`Player Possessed` :type "/Game/BallControl041/Blueprints/SoccerPlayer/BP_Player Object Reference"))
  (bind _outactors (`GameplayStatics.GetAllActorsOfClass` "/Game/BallControl041/Blueprints/SoccerPlayer/BP_Player.BP_Player_C"))
  (for _array_element _outactors
    (if (`/Game/BallControl041/Blueprints/SoccerPlayer/BP_Player.Player Possessed` _array_element)
      (return _array_element))))

(fn `Get Players OutBall`
  (returns (`Players OutBall` :type "/Game/BallControl041/Blueprints/SoccerPlayer/BP_Player Object Reference"))
  (bind _outactors (`GameplayStatics.GetAllActorsOfClass` "/Game/BallControl041/Blueprints/SoccerPlayer/BP_Player.BP_Player_C"))
  (for _array_element _outactors
    (if (not (`/Game/BallControl041/Blueprints/SoccerPlayer/BP_Player.Is withBall?` _array_element))
      (return _array_element))))

(fn `UserConstructionScript`)