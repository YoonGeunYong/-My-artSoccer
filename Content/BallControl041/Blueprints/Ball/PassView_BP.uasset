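; PassView_BP is a pass-target indicator that marks the player location supplied by PassGuide_BP.
; BeginPlay caches the first PassGuide_BP and BP_Ball found in the level.
; Each tick, while the ball has passing or crossing enabled and the guide's FollowGuide flag is set, it moves its FollowClosePlayer component to that location's X and Y at a fixed low height.
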(event `self.ReceiveBeginPlay`
  ;[1 1 1] Get Actors
  (bind _outactors (`GameplayStatics.GetAllActorsOfClass` "/Game/BallControl041/Blueprints/Ball/PassGuide_BP.PassGuide_BP_C"))
  (set `self.PassGuide BP` (`|GetArrayItem` _outactors))
  (bind _outactors_2 (`GameplayStatics.GetAllActorsOfClass` "/Game/BallControl041/Blueprints/Ball/BP_Ball.BP_Ball_C"))
  (set `self.Ball BP` (`|GetArrayItem` _outactors_2)))

(event `self.ReceiveTick`
  (params (DeltaSeconds :type "Float (single-precision)"))
  (`self.Follow ClosePlayer Event`))

(event `Follow ClosePlayer Event`
  (bind _ball_bp (`self.Ball BP`))
  ;[1 1 1] Get Player Location
  (if (or (`/Game/BallControl041/Blueprints/Ball/BP_Ball.Enable BallPass` _ball_bp) (`/Game/BallControl041/Blueprints/Ball/BP_Ball.Enable Crossing` _ball_bp))
    (set `self.Player_Location` (`/Game/BallControl041/Blueprints/Ball/PassGuide_BP.Player_Location` (`self.PassGuide BP`)))
    ;[1 1 1] "Follow_ClosePlayer" will follow "PlayerLocation"
    (bind _output_get (set `self.Follow_PassGuide` (`/Game/BallControl041/Blueprints/Ball/PassGuide_BP.FollowGuide` (`self.PassGuide BP`))))
    (if _output_get
      (`SceneComponent.K2_SetWorldLocation` (`self.Follow_ClosePlayer`) (`KismetMathLibrary.MakeVector` (.x (`self.Player_Location`)) (.y (`self.Player_Location`)) 4.0) false false))))

(fn `UserConstructionScript`)