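; Game mode for a two-team football match of players against goalkeepers, running login, spawning, scoring and the match clock.
; Once all expected players log in, it splits controllers by team parity, then spawns and possesses Blue players and Red goalkeepers at tagged starts.
; It relays start, goal and end events to every controller, with a timed unfreeze after each start.
; Goals respawn teams and ball; a looping timer counts GameState time down to the end.
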(event `self.ReceiveBeginPlay`
  (bind _outactors (`GameplayStatics.GetAllActorsOfClassWithTag` "/Script/Engine.PlayerStart" "GoalKeeperStart"))
  (set `self.BlueSpawn` _outactors)
  (bind _outactors_2 (`GameplayStatics.GetAllActorsOfClassWithTag` "/Script/Engine.PlayerStart" "KickerStart"))
  (set `self.RedSpawn` _outactors_2)
  (bind _asbp_gstate (cast `/Game/Content/Maps/GameMap/BP_Gstate` (`GameplayStatics.GetGameState`)))
  (bind _output_get (set `self.As BP Gstate` _asbp_gstate))
  (set `/Game/Content/Maps/GameMap/BP_Gstate.CurrentTime` (`self.Timer`) _output_get))

(event `InformAll`
  (params (What :type Integer) (Team :type Boolean))
  ;[1 1 1] ServerToAll
  (for _array_element (`self.PlayerList`)
    (bind _asbp_game_control (cast `/Game/Content/Maps/GameMap/BP_GameControl` _array_element))
    (`/Game/Content/Maps/GameMap/BP_GameControl.CallFromServer` _asbp_game_control Team What)))

(event `UnPause`
  (`self.UnFreeze`))

(event `UnFreeze`
  (for _array_element (`self.PlayerList`)
    (bind _asbp_game_control (cast `/Game/Content/Maps/GameMap/BP_GameControl` _array_element))
    (`/Game/Content/Maps/GameMap/BP_GameControl.UnFreeze` _asbp_game_control))
  (set `self.NotPaused` true))

(event `self.K2_PostLogin`
  (params (NewPlayer :type "PlayerController Object Reference"))
  (`KismetArrayLibrary.Array_Add` (`self.PlayerList`) NewPlayer)
  (bind _asbp_game_control (cast `/Game/Content/Maps/GameMap/BP_GameControl` NewPlayer))
  (`/Game/Content/Maps/GameMap/BP_GameControl.SetPlayerState` _asbp_game_control)
  (bind _result (`/Engine/EditorBlueprintResources/StandardMacros.IncrementInt` (`self.CurrentPlayers`))
    (:`  `
      (if (== _result (`/Game/Content/Blueprints/BP_GameInstance.Total` (cast `/Game/Content/Blueprints/BP_GameInstance` (`GameplayStatics.GetGameInstance`) :!pure true)))
        (`KismetSystemLibrary.Delay` 2.0)
        (for _array_element (`self.PlayerList`)
          (bind _asbp_player_state (cast `/Game/Content/Maps/Lobby/BP_PlayerState` (`Controller.PlayerState` _array_element)))
          (bind _asbp_game_control_2 (cast `/Game/Content/Maps/GameMap/BP_GameControl` _array_element))
          (if (== (mod (`/Game/Content/Maps/Lobby/BP_PlayerState.team` _asbp_player_state) 2) 0)
            (`KismetArrayLibrary.Array_Add` (`self.RedTeam`) _asbp_game_control_2)
            (else
              (`KismetArrayLibrary.Array_Add` (`self.BlueTeam`) _asbp_game_control_2))))
        (`KismetSystemLibrary.K2_SetTimerDelegate` (delegate `Count`) 1.0 true)
        (`self.StartGame` 0)))))

(event `StartGame`
  (params (What :type Integer) (Team :type Boolean))
  (`self.SpawnTeams`)
  (`self.InformAll` What Team)
  (bind _returnvalue (`KismetSystemLibrary.K2_SetTimer` null "UnPause" 3.0 false 1.0))
  (set `self.Handler` _returnvalue))

(event `EndGame`
  (`self.DeSpawnTeams`)
  (`self.InformAll` 2))

(event `Count`
  (if (`self.NotPaused`)
    (bind _result (`/Engine/EditorBlueprintResources/StandardMacros.DecrementInt` (`/Game/Content/Maps/GameMap/BP_Gstate.CurrentTime` (`self.As BP Gstate`)))
      (:`  `
        (if (== _result 0)
          (`self.EndGame`))))))

(event `Goal`
  (params (Team :type Boolean))
  (`self.DeSpawnTeams`)
  (`/Engine/EditorBlueprintResources/StandardMacros.IncrementInt` (select `bool` Team :`false` (`self.RedScore`) :`true` (`self.BlueScore`))
    (:`  `
      (`self.StartGame` 1 Team)
      (`|SpawnActorFromClass` "/Game/Content/Blueprints/BP_FootBall.BP_FootBall_C" (`KismetMathLibrary.MakeTransform` (0.0 0.0 600.0) (struct) (0.25 0.25 0.25)) "Undefined" "MultiplyWithRoot" null null))))

(fn `DeSpawnTeams`
  (for _array_element (`self.BlueTeam`)
    (bind _returnvalue (`Controller.K2_GetPawn` _array_element))
    (`/Engine/EditorBlueprintResources/StandardMacros.IsValid` _returnvalue
      (:`Is Valid`
        (`self.K2_DestroyActor` _returnvalue))))
  (for _array_element_2 (`self.RedTeam`)
    (bind _returnvalue_2 (`Controller.K2_GetPawn` _array_element_2))
    (`/Engine/EditorBlueprintResources/StandardMacros.IsValid` _returnvalue_2
      (:`Is Valid`
        (`self.K2_DestroyActor` _returnvalue_2)))))

(fn `SpawnTeams`
  (for (_array_element _array_index) (`self.BlueTeam`)
    (bind _returnvalue (`|SpawnActorFromClass` "/Game/BallControl041/Blueprints/SoccerPlayer/BP_Player.BP_Player_C" (`self.GetTransform` (`|GetArrayItem` (`self.BlueSpawn`) _array_index)) "Undefined" "MultiplyWithRoot" null null))
    (`Controller.Possess` _array_element _returnvalue))
  (for (_array_element_2 _array_index_2) (`self.RedTeam`)
    (bind _returnvalue_2 (`|SpawnActorFromClass` "/Game/BallControl041/Blueprints/SoccerPlayer/BP_GoalKeeper.BP_GoalKeeper_C" (`self.GetTransform` (`|GetArrayItem` (`self.RedSpawn`) _array_index_2)) "Undefined" "MultiplyWithRoot" null null))
    (`Controller.Possess` _array_element_2 _returnvalue_2)))

(fn `UserConstructionScript`)