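; Game mode for a local multiplayer soccer game that sets up players and their pawns at BeginPlay.
; It loops over every PlayerStart, calling CreatePlayer for its index and adding the default Enhanced Input mapping context for that player.
; The first start spawns a BP_GoalKeeper possessed by player 0, while each later start spawns a BP_Player possessed by the matching controller.
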(event `self.ReceiveBeginPlay`
  (bind _returnvalue (`GameplayStatics.GetPlayerController` 0))
  (bind _outactors (`GameplayStatics.GetAllActorsOfClass` "/Script/Engine.PlayerStart"))
  (for (_array_element _array_index) _outactors
    (bind _output_get (set `self.Array Index` _array_index))
    (bind _returnvalue_2 (`GameplayStatics.CreatePlayer` _output_get))
    (if (> (`self.Array Index`) 0)
      (`EnhancedInputSubsystemInterface.AddMappingContext` (pcsubsystem `EnhancedInputLocalPlayerSubsystem` _returnvalue_2) "/Game/ThirdPerson/Input/IMC_Default.IMC_Default" 0 (struct))
      (bind _returnvalue_3 (`self.GetTransform` _array_element))
      (bind _returnvalue_4 (`|SpawnActorFromClass` "/Game/BallControl041/Blueprints/SoccerPlayer/BP_Player.BP_Player_C" _returnvalue_3 "Undefined" "MultiplyWithRoot" null null))
      (`Controller.Possess` (`GameplayStatics.GetPlayerController` (`self.Array Index`)) _returnvalue_4)
      (else
        (`EnhancedInputSubsystemInterface.AddMappingContext` (pcsubsystem `EnhancedInputLocalPlayerSubsystem` _returnvalue) "/Game/ThirdPerson/Input/IMC_Default.IMC_Default" 0 (struct))
        (bind _returnvalue_5 (`|SpawnActorFromClass` "/Game/BallControl041/Blueprints/SoccerPlayer/BP_GoalKeeper.BP_GoalKeeper_C" _returnvalue_3 "Undefined" "MultiplyWithRoot" null null))
        (`Controller.Possess` _returnvalue _returnvalue_5)))))

(fn `UserConstructionScript`)