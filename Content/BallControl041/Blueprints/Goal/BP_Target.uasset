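; BP_Target is the aim marker for shots at goal, moving its Target component from stick and key input every Tick.
; During a ball free kick, input accumulates into clamped horizontal and height offsets, unless the ball carrier's LockGoalTarget is set.
; GetPlayer finds that carrier by scanning all BP_Player actors.
; Otherwise, the vertical input axis alone sets a world X position that the target eases toward with VInterpTo.
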(event `self.ReceiveTick`
  (params (DeltaSeconds :type "Float (single-precision)"))
  (bind _target (`self.Target`))
  (bind _target_2 (`self.Target`))
  (bind (_returnvalue_x _returnvalue_y) (`KismetMathLibrary.BreakVector` (`SceneComponent.K2_GetComponentLocation` _target)))
  (bind (_returnvalue_x_2 _returnvalue_y_2 _returnvalue_z) (`KismetMathLibrary.BreakVector` (`SceneComponent.K2_GetComponentLocation` _target_2)))
  (bind _returnvalue_x_3 (`KismetMathLibrary.BreakVector` (`KismetMathLibrary.MakeVector` (+ (`self.GetInputAxisValue`) (`self.GetInputAxisValue`)))))
  (bind _returnvalue_x_4 (`KismetMathLibrary.BreakVector` (`KismetMathLibrary.MakeVector` (+ (`self.GetInputAxisValue`) (`self.GetInputAxisValue`)))))
  (bind _returnvalue_x_5 (`KismetMathLibrary.BreakVector` (`KismetMathLibrary.MakeVector` (+ (`self.GetInputAxisValue`) (`self.GetInputAxisValue`)))))
  ;[1 1 1] (Free Kick) Get Vertical and Horizontal Input to Control the (Target)
  (if (`/Game/BallControl041/Blueprints/Ball/BP_Ball.FreeKick` (`self.Ball BP`))
    (bind _player (`self.Get Player`))
    (if (not (`/Game/BallControl041/Blueprints/SoccerPlayer/BP_Player.Lock Goal Target` _player))
      (bind _output_get (set `self.Vertical` (`KismetMathLibrary.FClamp` (+ (`self.Vertical`) (* _returnvalue_x_5 10.0)) -60.0 150.0)))
      (bind _output_get_2 (set `self.Horizontal` (`KismetMathLibrary.FClamp` (+ (`self.Horizontal`) (* _returnvalue_x_3 -10.0)) -350.0 350.0)))
      ;[1 1 1] Set (Target) Location to be controlled by Input
      (`SceneComponent.K2_SetWorldLocation` _target (`KismetMathLibrary.MakeVector` _output_get_2 _returnvalue_y (+ _output_get 90.0)) false false))
    (else
      ;[1 1 1] Vertical Input
      (bind _output_get_3 (set `self.Horizontal` _returnvalue_x_4))
      ;[1 1 1] Set (Target) Location to Input
      (`SceneComponent.K2_SetWorldLocation` _target_2 (`KismetMathLibrary.VInterpTo` (`SceneComponent.K2_GetComponentLocation` _target_2) (`KismetMathLibrary.MakeVector` (* _output_get_3 300.0) _returnvalue_y_2 _returnvalue_z) (`GameplayStatics.GetWorldDeltaSeconds`) 4.0) false false))))

(fn `Get Player`
  (returns (Player :type "/Game/BallControl041/Blueprints/SoccerPlayer/BP_Player Object Reference"))
  (bind _outactors (`GameplayStatics.GetAllActorsOfClass` "/Game/BallControl041/Blueprints/SoccerPlayer/BP_Player.BP_Player_C"))
  (for _array_element _outactors
    (if (`/Game/BallControl041/Blueprints/SoccerPlayer/BP_Player.Is withBall?` _array_element)
      (return _array_element))))

(fn `UserConstructionScript`)