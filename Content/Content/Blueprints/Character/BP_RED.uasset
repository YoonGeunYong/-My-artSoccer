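; BP_RED is a playable third-person football character for multiplayer, with Enhanced Input movement, camera look and jumping.
; HitRange overlaps track the nearby ball, which side passes, upward kicks and forward kicks (lofted unless Left Ctrl is held) send through CallToServer to RPCPass, scaled by a cyclable Power.
; Sprint sets speed locally and through server events.
; The GameInstance username feeds a name tag via OnRep, which retries until the widget exists.
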(event `self.ReceiveBeginPlay`
  (bind _returnvalue (pcsubsystem `EnhancedInputLocalPlayerSubsystem` (`GameplayStatics.GetPlayerController` 0)))
  (`/Engine/EditorBlueprintResources/StandardMacros.IsValid` _returnvalue
    (:`Is Valid`
      (`EnhancedInputSubsystemInterface.AddMappingContext` _returnvalue "/Game/Content/Input/INC_ThirdPerson.INC_ThirdPerson" 0 (struct)))))

(event `SetPlayerNameOnServer`
  (params (CustomPlayerName :type Text))
  (set `self.CustomPlayerName` CustomPlayerName))

(event `EnhancedInput|/Game/Content/Input/Actions/INP_Jump`
  (params (ActionValue :type Boolean) (ElapsedSeconds :type "Float (double-precision)") (TriggeredSeconds :type "Float (double-precision)") (InputAction :type "InputAction Object Reference" :default "/Game/Content/Input/Actions/INP_Jump.INP_Jump"))
  (:`Started`
    (`self.Jump`))
  (:`Completed`
    (`self.StopJumping`)))

(event `EnhancedInput|/Game/Content/Input/Actions/INP_MoveAround`
  (params (ActionValue :type "Vector2D Structure") (ElapsedSeconds :type "Float (double-precision)") (TriggeredSeconds :type "Float (double-precision)") (InputAction :type "InputAction Object Reference" :default "/Game/Content/Input/Actions/INP_MoveAround.INP_MoveAround"))
  (bind (_returnvalue_roll _returnvalue_pitch _returnvalue_yaw) (`KismetMathLibrary.BreakRotator` (`self.GetControlRotation`)))
  (:`Triggered`
    (`self.AddMovementInput` (`KismetMathLibrary.GetRightVector` (`self.GetControlRotation`)) ActionValue_X)
    (`self.AddMovementInput` (`KismetMathLibrary.GetForwardVector` (`KismetMathLibrary.MakeRotator` _returnvalue_roll 0.0 _returnvalue_yaw)) ActionValue_Y)))

(event `EnhancedInput|/Game/Content/Input/Actions/INP_LookAround`
  (params (ActionValue :type "Vector2D Structure") (ElapsedSeconds :type "Float (double-precision)") (TriggeredSeconds :type "Float (double-precision)") (InputAction :type "InputAction Object Reference" :default "/Game/Content/Input/Actions/INP_LookAround.INP_LookAround"))
  (:`Triggered`
    (`self.AddControllerYawInput` (* ActionValue_X (`KismetMathLibrary.SelectFloat` -1.0 1.0 (`self.InvertCameraX`))))
    (`self.AddControllerPitchInput` (* ActionValue_Y (`KismetMathLibrary.SelectFloat` -1.0 1.0 (`self.InvertCameraY`))))))

(event `self.HitRange.OnComponentBeginOverlap`
  (params (OverlappedComponent :type "PrimitiveComponent Object Reference") (OtherActor :type "Actor Object Reference") (OtherComp :type "PrimitiveComponent Object Reference") (OtherBodyIndex :type Integer) (bFromSweep :type Boolean) (SweepResult :type "HitResult Structure (by ref)"))
  (bind _asbp_foot_ball (cast `/Game/Content/Blueprints/BP_FootBall` OtherActor))
  (set `self.BallObject` _asbp_foot_ball))

(event `self.HitRange.OnComponentEndOverlap`
  (params (OverlappedComponent :type "PrimitiveComponent Object Reference") (OtherActor :type "Actor Object Reference") (OtherComp :type "PrimitiveComponent Object Reference") (OtherBodyIndex :type Integer))
  (cast `/Game/Content/Blueprints/BP_FootBall` OtherActor)
  (set `self.BallObject` null))

(event `EnhancedInput|/Game/Content/Input/Actions/INP_Power`
  (params (ActionValue :type "Float (double-precision)") (ElapsedSeconds :type "Float (double-precision)") (TriggeredSeconds :type "Float (double-precision)") (InputAction :type "InputAction Object Reference" :default "/Game/Content/Input/Actions/INP_Power.INP_Power"))
  (bind _returnvalue (+ (select `bool` (< ActionValue 0.0) :`false` 30.0 :`true` -30.0) (`self.Power`)))
  (bind _returnvalue_2 (< _returnvalue 30.0))
  (:`Triggered`
    (if (or _returnvalue_2 (> _returnvalue 90.0))
      (if _returnvalue_2
        (bind _output_get (set `self.Power` 90.0))
        (`KismetSystemLibrary.PrintString` (`KismetStringLibrary.Conv_DoubleToString` _output_get))
        (else
          (bind _output_get_2 (set `self.Power` 30.0))
          (`KismetSystemLibrary.PrintString` (`KismetStringLibrary.Conv_DoubleToString` _output_get_2))))
      (else
        (bind _output_get_3 (set `self.Power` _returnvalue))
        (`KismetSystemLibrary.PrintString` (`KismetStringLibrary.Conv_DoubleToString` _output_get_3))))))

(event `EnhancedInput|/Game/Content/Input/Actions/INP_Right`
  (params (ActionValue :type Boolean) (ElapsedSeconds :type "Float (double-precision)") (TriggeredSeconds :type "Float (double-precision)") (InputAction :type "InputAction Object Reference" :default "/Game/Content/Input/Actions/INP_Right.INP_Right"))
  (bind _power (`self.Power`))
  (:`Triggered`
    (`self.CallToServer` (`KismetMathLibrary.GetUpVector` (`self.GetControlRotation`)) (+ _power (* (+ (/ _power 30.0) -1.0) -20.0)))))

(event `Key|LeftControl`
  (params (Key :type "Key Structure"))
  (:`Pressed`
    (set `self.Over` true))
  (:`Released`
    (set `self.Over` false)))

(event `CallToServer`
  (params (Direction :type "Vector Structure") (Power :type "Float (double-precision)"))
  (bind _ballobject (`self.BallObject`)
    (:`then`
      (`/Game/Content/Blueprints/BP_FootBall.RPC_Pass` _ballobject Direction Power))
    (:`else`)))

(event `EnhancedInput|/Game/Content/Input/Actions/INP_PassLeft`
  (params (ActionValue :type Boolean) (ElapsedSeconds :type "Float (double-precision)") (TriggeredSeconds :type "Float (double-precision)") (InputAction :type "InputAction Object Reference" :default "/Game/Content/Input/Actions/INP_PassLeft.INP_PassLeft"))
  (:`Triggered`
    (`self.CallToServer` (* -1.0 (`KismetMathLibrary.GetRightVector` (`self.GetControlRotation`))) (/ (`self.Power`) 10.0))))

(event `EnhancedInput|/Game/Content/Input/Actions/INP_PassRight`
  (params (ActionValue :type Boolean) (ElapsedSeconds :type "Float (double-precision)") (TriggeredSeconds :type "Float (double-precision)") (InputAction :type "InputAction Object Reference" :default "/Game/Content/Input/Actions/INP_PassRight.INP_PassRight"))
  (:`Triggered`
    (`self.CallToServer` (`KismetMathLibrary.GetRightVector` (`self.GetControlRotation`)) (/ (`self.Power`) 10.0))))

(event `Key|LeftShift`
  (params (Key :type "Key Structure"))
  (bind _charactermovement (`self.CharacterMovement`))
  (:`Pressed`
    (`self.ServerSprint`)
    (set `self.Sprinting` true)
    (set `CharacterMovementComponent.MaxWalkSpeed` 750.0 _charactermovement))
  (:`Released`
    (`self.ServerWalk`)
    (set `self.Sprinting` false)
    (set `CharacterMovementComponent.MaxWalkSpeed` 600.0 _charactermovement)))

(event `ServerSprint`
  (set `self.Sprinting` true)
  (set `CharacterMovementComponent.MaxWalkSpeed` 750.0 (`self.CharacterMovement`)))

(event `ServerWalk`
  (set `self.Sprinting` false)
  (set `CharacterMovementComponent.MaxWalkSpeed` 600.0 (`self.CharacterMovement`)))

(event `EnhancedInput|/Game/Content/Input/Actions/INP_Left`
  (params (ActionValue :type Boolean) (ElapsedSeconds :type "Float (double-precision)") (TriggeredSeconds :type "Float (double-precision)") (InputAction :type "InputAction Object Reference" :default "/Game/Content/Input/Actions/INP_Left.INP_Left"))
  (bind (_returnvalue_x _returnvalue_y _returnvalue_z) (`KismetMathLibrary.BreakVector` (`self.GetActorForwardVector`)))
  (:`Triggered`
    (`self.CallToServer` (`KismetMathLibrary.MakeVector` _returnvalue_x _returnvalue_y (select `bool` (`self.Over`) :`false` 0.395 :`true` _returnvalue_z)) (+ 35.0 (* (/ (`self.Power`) 100.0) 30.0)))))

(fn `OnRep_CustomPlayerName`
  (bind _returnvalue (`WidgetComponent.GetWidget` (`self.PlayerNameTagWidget`)))
  (`/Engine/EditorBlueprintResources/StandardMacros.IsValid` _returnvalue
    (:`Is Valid`
      (bind _asname_tag (cast `/Game/Content/UI/NameTag` _returnvalue))
      (`/Game/Content/UI/NameTag.SetPlayerName` _asname_tag (`self.CustomPlayerName`))
      (`SceneComponent.SetHiddenInGame` (`self.PlayerNameTagWidget`) false false))
    (:`Is Not Valid`
      (`KismetSystemLibrary.K2_SetTimer` null "OnRep_CustomPlayerName" 0.1))))

(fn `SetUpLocal`
  (if (`self.IsLocallyControlled`)
    (`self.SetPlayerNameOnServer` (`/Game/Content/Blueprints/BP_GameInstance.Username` (cast `/Game/Content/Blueprints/BP_GameInstance` (`GameplayStatics.GetGameInstance`) :!pure true)))))

(fn `UserConstructionScript`)