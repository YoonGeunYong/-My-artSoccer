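; BP_LobbyCtrl is the lobby controller that sets up each player's UI and identity and handles map travel.
; SetPlayerState creates the UI_Lobby widget, saves the team to the game instance, then writes username and team to BP_PlayerState, retrying each second until the cast succeeds.
; UpdateWidget refreshes the lobby UI after a short delay, and MapTravel issues a serverTravel console command.
; A debug key prints every player's team and username.
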(event `SetPlayerState`
  (params (team :type Integer))
  (bind _asbp_game_instance (cast `/Game/Content/Blueprints/BP_GameInstance` (`GameplayStatics.GetGameInstance`) :!pure true))
  (bind _returnvalue (`|CreateWidget` "/Game/Content/UI/UI_Lobby.UI_Lobby_C"))
  (bind _output_get (set `self.Lobby` _returnvalue))
  (`UserWidget.AddToViewport` _output_get 0)
  (set `/Game/Content/Blueprints/BP_GameInstance.TeamPlayerNo` team _asbp_game_instance)
  (`self.SetState` (`/Game/Content/Blueprints/BP_GameInstance.Username` _asbp_game_instance) team))

(event `SetState`
  (params (username :type Text) (team :type Integer))
  (bind _asbp_player_state (cast `/Game/Content/Maps/Lobby/BP_PlayerState` (`self.PlayerState`) :!label _label)
    (:`then`
      (set `/Game/Content/Maps/Lobby/BP_PlayerState.username` username _asbp_player_state)
      (set `/Game/Content/Maps/Lobby/BP_PlayerState.team` team _asbp_player_state))
    (:`CastFailed`
      (`KismetSystemLibrary.Delay` 1.0)
      (goto _label))))

(event `UpdateWidget`
  (`KismetSystemLibrary.Delay` 1.0)
  (`/Game/Content/UI/UI_Lobby.UpdateWidget` (`self.Lobby`)))

(event `MapTravel`
  (params (MapName :type String))
  (`KismetSystemLibrary.ExecuteConsoleCommand` (`KismetStringLibrary.Concat_StrStr` "serverTravel " MapName) null))

(event `Key|A`
  (params (Key :type "Key Structure"))
  (:`Pressed`
    (bind _asbp_lobby_state (cast `/Game/Content/Maps/Lobby/BP_LobbyState` (`GameplayStatics.GetGameState`)))
    (for _array_element (`GameStateBase.PlayerArray` _asbp_lobby_state)
      (bind _asbp_player_state (cast `/Game/Content/Maps/Lobby/BP_PlayerState` _array_element))
      (`KismetSystemLibrary.PrintString` (`KismetTextLibrary.Conv_TextToString` (`|FormatText` "Team {team} , username {username}" (`/Game/Content/Maps/Lobby/BP_PlayerState.team` _asbp_player_state) (`/Game/Content/Maps/Lobby/BP_PlayerState.username` _asbp_player_state)))))))

(fn `UserConstructionScript`)