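; Player-controlled goalkeeper Character that moves sideways along world Y and jumps.
; Enhanced Input drives movement, while jumping uses LaunchCharacter, keeping Y velocity and launching lower at high lateral speed.
; A ground flag gates jumps, clearing on launch and resetting when the capsule hits an actor tagged "Ground".
; Ball overlap only prints a debug string, and Tick stores whether move input is ignored.
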(event `self.ReceiveTick`
  (params (DeltaSeconds :type "Float (single-precision)"))
  (set `self.IsMove` (`PawnMovementComponent.IsMoveInputIgnored` (`self.CharacterMovement`))))

(event `EnhancedInput|/Game/Content/Input/Actions/INP_Jump`
  (params (ActionValue :type Boolean) (ElapsedSeconds :type "Float (double-precision)") (TriggeredSeconds :type "Float (double-precision)") (InputAction :type "InputAction Object Reference" :default "/Game/Content/Input/Actions/INP_Jump.INP_Jump"))
  (bind (_returnvalue_x _returnvalue_y) (`KismetMathLibrary.BreakVector` (`self.GetVelocity`)))
  (:`Started`
    (if (`self.IsGround`)
      (`self.LaunchCharacter` (`KismetMathLibrary.MakeVector` 0.0 _returnvalue_y (select `bool` (or (> _returnvalue_y 575.0) (< _returnvalue_y -575.0)) :`false` 600.0 :`true` 300.0)))
      (set `self.IsGround` false))))

(event `self.CapsuleComponent.OnComponentBeginOverlap`
  (params (OverlappedComponent :type "PrimitiveComponent Object Reference") (OtherActor :type "Actor Object Reference") (OtherComp :type "PrimitiveComponent Object Reference") (OtherBodyIndex :type Integer) (bFromSweep :type Boolean) (SweepResult :type "HitResult Structure (by ref)"))
  (cast `/Game/BallControl041/Blueprints/Ball/BP_Ball` OtherActor)
  (`KismetSystemLibrary.PrintString` "Hello"))

(event `EnhancedInput|/Game/Content/Input/Actions/INP_MoveAround`
  (params (ActionValue :type "Vector2D Structure") (ElapsedSeconds :type "Float (double-precision)") (TriggeredSeconds :type "Float (double-precision)") (InputAction :type "InputAction Object Reference" :default "/Game/Content/Input/Actions/INP_MoveAround.INP_MoveAround"))
  (:`Triggered`
    (bind _output_get (set `self.Horizontal` ActionValue_X))
    (`self.AddMovementInput` (`KismetMathLibrary.GetRightVector` (struct)) _output_get)))

(event `self.CapsuleComponent.OnComponentHit`
  (params (HitComponent :type "PrimitiveComponent Object Reference") (OtherActor :type "Actor Object Reference") (OtherComp :type "PrimitiveComponent Object Reference") (NormalImpulse :type "Vector Structure") (Hit :type "HitResult Structure (by ref)"))
  (if (`self.ActorHasTag` OtherActor "Ground")
    (set `self.IsGround` true)))

(fn `UserConstructionScript`
  (`parent.UserConstructionScript`))