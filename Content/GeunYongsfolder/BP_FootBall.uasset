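; Soccer ball actor that handles possession and passing between BP_Player characters.
; When HitField overlaps a player outside a shot, the nearest player becomes owner, with short steal delays, and the ball stops at their feet.
; An ownership change makes player controller 0 possess the new owner and gives the initially controlled pawn an AI controller once left.
; Passes apply a velocity-change impulse, with an authority-checked RPC_Pass entry point.
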(event `RPC_Pass`
  (params (Direction :type "Vector Structure") (Power :type "Float (double-precision)"))
  (`/Engine/EditorBlueprintResources/ActorMacros.Switch Has Authority`
    (:`Authority`
      (`self.Pass` Direction Power))))

(event `Pass`
  (params (Direction :type "Vector Structure") (Power :type "Float (double-precision)"))
  (`PrimitiveComponent.AddImpulse` (`self.FootBall`) (* Direction Power (`self.ExtraSpeed`)) "None" true))

(event `self.ReceiveBeginPlay`
  (bind _outactors (`GameplayStatics.GetAllActorsOfClass` "/Game/Content/Blueprints/Character/BP_Player.BP_Player_C"))
  (set `self.Players` _outactors)
  (set `self.FirstOwner'sPawn` (`Controller.K2_GetPawn` (`GameplayStatics.GetPlayerController` 0))))

(event `self.HitField.OnComponentBeginOverlap`
  (params (OverlappedComponent :type "PrimitiveComponent Object Reference") (OtherActor :type "Actor Object Reference") (OtherComp :type "PrimitiveComponent Object Reference") (OtherBodyIndex :type Integer) (bFromSweep :type Boolean) (SweepResult :type "HitResult Structure (by ref)"))
  (bind _ownerplayer (`self.OwnerPlayer`))
  (bind (_distance _returnvalue) (`GameplayStatics.FindNearestActor` (`self.K2_GetActorLocation`) (`self.Players`)))
  (if (not (`self.Shooting`))
    (cast `/Game/Content/Blueprints/Character/BP_Player` OtherActor)
    (if (== (`self.OwnerPlayer`) _returnvalue)
      (`self.K2_SetActorLocation` self (+ (`self.K2_GetActorLocation` _ownerplayer) (* (`self.GetActorForwardVector` _ownerplayer) (75.0 75.0 0.0)) (0.0 0.0 -50.0)) false false :!label _label)
      (`PrimitiveComponent.SetPhysicsLinearVelocity` (`self.FootBall`) (0.0 0.0 0.0) false "None")
      (else
        (if (not (`self.CanSteelTheBall`))
          (`KismetSystemLibrary.Delay` 0.5))
        (`/Engine/EditorBlueprintResources/StandardMacros.IsValid` _ownerplayer
          (:`Is Valid`
            (set `self.ActorBeforeChange` _ownerplayer))
          (:`Is Not Valid`
            _))
        (bind _output_get (set `self.OwnerPlayer` _returnvalue))
        (bind _aspawn (cast `Pawn` _output_get))
        (`Controller.Possess` (`GameplayStatics.GetPlayerController` 0) _aspawn)
        (`self.CreateFristPlayerAIController` (== (`self.ActorBeforeChange`) (`self.FirstOwner'sPawn`)))
        (set `self.CanSteelTheBall` false)
        (`|ExecutionSequence`
          (:`then_0`
            (goto _label))
          (:`then_1`
            (`KismetSystemLibrary.Delay` 0.1)
            (set `self.CanSteelTheBall` true)))))))

(fn `CreateFristPlayerAIController`
  (params (Condition :type Boolean))
  (bind _instigator (`Actor.Instigator` (`self.FirstOwner'sPawn`)))
  (set `self.FirstActorChanging` true)
  (if Condition
    (`Pawn.SpawnDefaultController` _instigator)
    (bind _asbp_aicontroller (cast `/Game/Content/Blueprints/BP_AIController` (`Pawn.GetController` _instigator)))
    (set `/Game/Content/Blueprints/BP_AIController.MyPawn` _instigator _asbp_aicontroller)
    (set `self.FirstOwner'sPawn` null)))

(fn `UserConstructionScript`)