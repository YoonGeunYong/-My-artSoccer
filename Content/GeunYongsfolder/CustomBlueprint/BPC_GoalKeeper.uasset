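; Player-controlled goalkeeper character that slides sideways along world Y and jumps, kept within fixed bounds on that axis.
; Move input adds sideways movement inside the bounds; both Tick and the input handler offset the actor back when it reaches or passes a limit.
; Jump launches only when grounded, lower at high lateral speed, and hits on Ground-tagged actors restore the grounded flag.
; Capsule overlap casts to BP_Ball but does nothing further.
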(event `self.ReceiveTick`
  (params (DeltaSeconds :type "Float (single-precision)"))
  (bind (_returnvalue_x _returnvalue_y) (`KismetMathLibrary.BreakVector` (`self.K2_GetActorLocation`)))
  (bind _returnvalue (`KismetMathLibrary.FClamp` _returnvalue_y -350.0 350.0))
  (if (or (>= _returnvalue_y 350.0) (<= _returnvalue_y -350.0))
    (`self.K2_AddActorWorldOffset` (`KismetMathLibrary.MakeVector` 0.0 (`KismetMathLibrary.SelectFloat` (+ _returnvalue _returnvalue_y) (- _returnvalue _returnvalue_y))))))

(event `EnhancedInput|/Game/GeunYongsfolder/Input/Actions/INP_Jump`
  (params (ActionValue :type Boolean) (ElapsedSeconds :type "Float (double-precision)") (TriggeredSeconds :type "Float (double-precision)") (InputAction :type "InputAction Object Reference" :default "/Game/GeunYongsfolder/Input/Actions/INP_Jump.INP_Jump"))
  (bind (_returnvalue_x _returnvalue_y) (`KismetMathLibrary.BreakVector` (`self.GetVelocity`)))
  (:`Started`
    (if (`self.IsGround`)
      (`self.LaunchCharacter` (`KismetMathLibrary.MakeVector` 0.0 _returnvalue_y (select `bool` (or (> _returnvalue_y 575.0) (< _returnvalue_y -575.0)) :`false` 600.0 :`true` 300.0)))
      (set `self.IsGround` false))))

(event `self.CapsuleComponent.OnComponentBeginOverlap`
  (params (OverlappedComponent :type "PrimitiveComponent Object Reference") (OtherActor :type "Actor Object Reference") (OtherComp :type "PrimitiveComponent Object Reference") (OtherBodyIndex :type Integer) (bFromSweep :type Boolean) (SweepResult :type "HitResult Structure (by ref)"))
  (cast `/Game/BallControl041/Blueprints/Ball/BP_Ball` OtherActor))

(event `EnhancedInput|/Game/GeunYongsfolder/Input/Actions/INP_MoveAround`
  (params (ActionValue :type "Vector2D Structure") (ElapsedSeconds :type "Float (double-precision)") (TriggeredSeconds :type "Float (double-precision)") (InputAction :type "InputAction Object Reference" :default "/Game/GeunYongsfolder/Input/Actions/INP_MoveAround.INP_MoveAround"))
  (bind (_returnvalue_x _returnvalue_y _returnvalue_z) (`KismetMathLibrary.BreakVector` (`self.GetVelocity`)))
  (bind (_returnvalue_x_2 _returnvalue_y_2) (`KismetMathLibrary.BreakVector` (`self.K2_GetActorLocation`)))
  (bind _returnvalue (`KismetMathLibrary.FClamp` _returnvalue_y_2 -350.0 350.0))
  (:`Triggered`
    (bind _output_get (set `self.Horizontal` ActionValue_X))
    (if (and (>= _returnvalue_y_2 -350.0) (<= _returnvalue_y_2 350.0))
      (`self.AddMovementInput` (`KismetMathLibrary.GetRightVector` (struct)) _output_get)
      (else
        (`self.K2_AddActorWorldOffset` (`KismetMathLibrary.MakeVector` 0.0 (`KismetMathLibrary.SelectFloat` (+ _returnvalue _returnvalue_y_2) (- _returnvalue _returnvalue_y_2))) false true)
        (`PrimitiveComponent.SetPhysicsLinearVelocity` (`self.CapsuleComponent`) (`KismetMathLibrary.MakeVector` 0.0 0.0 _returnvalue_z) false "None")))))

(event `self.CapsuleComponent.OnComponentHit`
  (params (HitComponent :type "PrimitiveComponent Object Reference") (OtherActor :type "Actor Object Reference") (OtherComp :type "PrimitiveComponent Object Reference") (NormalImpulse :type "Vector Structure") (Hit :type "HitResult Structure (by ref)"))
  (if (`self.ActorHasTag` OtherActor "Ground")
    (set `self.IsGround` true)))

(fn `UserConstructionScript`
  (`parent.UserConstructionScript`))